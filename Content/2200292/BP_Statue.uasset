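; BP_Statue is a collectible that jumps to random positions in the level until the player's pawn touches it.
; InitStatue teleports it within fixed bounds and re-arms its own timer, with a delay that shrinks as the game mode's Level rises.
; On player overlap, unless the game is over, it notifies the game mode, destroys itself and spawns a replacement that randomizes its position on BeginPlay.
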(event EventBeginPlay
  (bind _asgame_mode (Utilities|Casting|CastToGameMODE (Game|GetGameMode)))
  (Variables|Default|SetAs%20BP%20Game%20Mode%20Lab%204 _asgame_mode)
  (CallFunction|InitStatue))

(event Collision|EventActorBeginOverlap
  (params (OtherActor :type Actor%20Object%20Reference))
  (if (and (== OtherActor (Game|Player|GetPlayerPawn 0)) (not (Variables|/Game/2200292/GameMODE.GameMODE_C|Getgameover (Variables|Default|GetAs%20BP%20Game%20Mode%20Lab%204))))
    (Default|StatueCollected (Variables|Default|GetAs%20BP%20Game%20Mode%20Lab%204))
    (Actor|DestroyActor)
    (Game|SpawnActorfromClass "BP_Statue_C" (Transformation|GetActorTransform (Variables|Default|GetAs%20BP%20Game%20Mode%20Lab%204)) "Undefined" "MultiplyWithRoot" 0 0)))

(fn ConstructionScript)

(fn InitStatue
  (Transformation|Teleport (Math|Vector|MakeVector (Math|Random|RandomFloatinRange 0.0 3.2e+03) (Math|Random|RandomFloatinRange 2e+02 3.2e+03) (Math|Random|RandomFloatinRange 0.0 1.8e+02)) "0, 0, 0")
  (Utilities|Time|SetTimerbyFunctionName 0 "InitStatue" (Math|Conversions|ToFloat(Integer) (- 6 (Variables|/Game/2200292/GameMODE.GameMODE_C|GetLevel (Variables|Default|GetAs%20BP%20Game%20Mode%20Lab%204))))))